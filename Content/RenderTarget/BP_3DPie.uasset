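; 3D pie or donut chart actor, rendered by a SceneCapture to a render target and handed out as a dynamic UI material.
; InitSegement builds one vertex-colored procedural mesh per data entry, sized by percentage and height, using translucent material when alpha is below one.
; MouseTrace deprojects the cursor through the capture camera, highlighting and offsetting the hit slice via material parameters.
; NotifyElementTipsLoc passes slice tip positions and camera info out.
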(event Custom|MouseTrace
  (params (MousePercentage :type Vector%202D%20Structure) (MousePos :type Vector%202D%20Structure) (ScreenSize :type Vector%202D%20Structure))
  (bind (_x _y) (Math|Vector2D|BreakVector2D ScreenSize))
  (bind (_x_2 _y_2) (Math|Vector2D|BreakVector2D MousePercentage))
  (bind _scenecapturecomponent2d (Variables|Default|GetSceneCaptureComponent2D))
  (bind _hoverinterval (Variables|半径|GethoverInterval))
  (bind _returnvalue (> _y 0.0))
  (bind _returnvalue_2 (/ _x _y))
  (bind _returnvalue_3 (Math|Float|SelectFloat _returnvalue_2 1.0 _returnvalue))
  (bind _minimalviewinfo (CallFunction|GetCameraMinimalViewInfo _returnvalue_3))
  (bind (_worldorigin _worlddirection) (Class|TransfromUtil|ScreentoWorld MousePos _minimalviewinfo ScreenSize _scenecapturecomponent2d))
  (if (and (Math|Float|InRange(Float) _x_2 -1.0 1.0) (Math|Float|InRange(Float) _y_2 -1.0 1.0))
    (bind _outhit (Collision|LineTraceForObjects _worldorigin (+ _worldorigin (* _worlddirection 1e+08)) (Utilities|Array|MakeArray "ObjectTypeQuery2" "ObjectTypeQuery1") false 0 "ForOneFrame" false))
    (bind _asprocedural_mesh_component (Utilities|Casting|CastToProceduralMeshComponent (.HitComponent (Collision|BreakHitResult _outhit)))
      (:then
        (bind _asmaterial_instance_dynamic (Utilities|Casting|CastToMaterialInstanceDynamic (Rendering|Material|GetMaterial _asprocedural_mesh_component 0))
          (:then
            (if (!= _asmaterial_instance_dynamic (Variables|缓存|GetLastMat))
              (Utilities|FlowControl|Sequence
                (:then_0
                  (Utilities|IsValid (Variables|缓存|GetLastMat)
                    (:Is%20Valid
                      (Rendering|Material|SetScalarParameterValue (Variables|缓存|GetLastMat) "Hover" 0.0 :!class /Script/Engine.MaterialInstanceDynamic)
                      (Rendering|Material|SetVectorParameterValue :self (Variables|缓存|GetLastMat) :ParameterName "Offset" :!class /Script/Engine.MaterialInstanceDynamic))))
                (:then_1
                  (Variables|缓存|SetLastMat _asmaterial_instance_dynamic)
                  (Variables|Default|SetLastComp _asprocedural_mesh_component)
                  (Rendering|Material|SetScalarParameterValue _asmaterial_instance_dynamic "Hover" 1.0 :!class /Script/Engine.MaterialInstanceDynamic)
                  (Rendering|Material|SetVectorParameterValue _asmaterial_instance_dynamic "Offset" (Utilities|Struct|MakeLinearColor (* _hoverinterval (Math|Trig|Sin(Degrees) (.Value (Utilities|Map|Find (Variables|缓存|GetcompsDegreeCenter) _asprocedural_mesh_component)))) (* (Math|Trig|Cos(Degrees) (.Value (Utilities|Map|Find (Variables|缓存|GetcompsDegreeCenter) _asprocedural_mesh_component))) _hoverinterval) 0.0 1.0) :!class /Script/Engine.MaterialInstanceDynamic)))))
          (:CastFailed
            (Utilities|IsValid (Variables|缓存|GetLastMat) :!label _label
              (:Is%20Valid
                (Rendering|Material|SetScalarParameterValue (Variables|缓存|GetLastMat) "Hover" 0.0 :!class /Script/Engine.MaterialInstanceDynamic)
                (Rendering|Material|SetVectorParameterValue :self (Variables|缓存|GetLastMat) :ParameterName "Offset" :!class /Script/Engine.MaterialInstanceDynamic)
                (Variables|缓存|SetLastMat 0)
                (Variables|Default|SetLastComp 0))))))
      (:CastFailed
        (goto _label)))))

(event EventBeginPlay
  (Utilities|FlowControl|Sequence
    (:then_0
      (bind _returnvalue (CanvasRenderTarget2D|CreateCanvasRenderTarget2D "/Script/Engine.CanvasRenderTarget2D" 1024 (Math|Float|Truncate (/ 1024.0 (Variables|缓存|GetaspectRatio)))))
      (Rendering|ClearRenderTarget2D _returnvalue)
      (Variables|/Script/Engine.SceneCaptureComponent2D|SetTextureTarget (Variables|Default|GetSceneCaptureComponent2D) _returnvalue)
      (bind _returnvalue_2 (Rendering|Material|CreateDynamicMaterialInstance "/Game/RenderTarget/M_CanvasRenderTarget2D.M_CanvasRenderTarget2D" "None" "None" :!class /Script/Engine.KismetMaterialLibrary))
      (Rendering|Material|SetTextureParameterValue _returnvalue_2 "Texture" _returnvalue)
      (Utilities|FlowControl|Delay 0.1)
      (Default|CallOnGetDynamicUIMaterial _returnvalue_2))
    (:then_1
      (CallFunction|InitSegement (Variables|缓存|GetData))
      (Rendering|SceneCapture|ShowOnlyActorComponents (Variables|Default|GetSceneCaptureComponent2D) self false)
      (Utilities|FlowControl|Delay 0.1)
      (CallFunction|NotifyElementTipsLoc))
    (:then_2
      (Collision|SetActorEnableCollision false))))

(event EventEndPlay
  (params (EndPlayReason :type EEndPlayReason%20Enum :default "Destroyed"))
  (bind _compsdegreecenter (Variables|缓存|GetcompsDegreeCenter))
  (bind _keys (Utilities|Map|Keys _compsdegreecenter))
  (Components|DestroyComponent _keys)
  (Utilities|Map|Clear _compsdegreecenter))

(fn ConstructionScript)

(fn CosA
  (params (angle :type Float%20%28single-precision%29))
  (return (* (Math|Trig|Cos(Degrees) angle) (Variables|半径|Getouter))))

(fn SinA
  (params (angle :type Float%20%28single-precision%29))
  (return (* (Math|Trig|Sin(Degrees) angle) (Variables|半径|Getouter))))

(fn GetSegmentTraingleList
  (params (bIsFirstSegment :type Boolean) (bIsLastSegment :type Boolean))
  (bind _anglestep (Variables|角度|GetangleStep))
  (bind _angle (Variables|角度|Getangle))
  (bind _angle_2 (Variables|角度|Getangle))
  (bind _anglestep_2 (Variables|角度|GetangleStep))
  (bind _angle_3 (Variables|角度|Getangle))
  (bind _inner (Variables|半径|Getinner))
  (bind _inner_2 (Variables|半径|Getinner))
  (bind _inner_3 (Variables|半径|Getinner))
  (bind _inner_4 (Variables|半径|Getinner))
  (bind _angle_4 (Variables|角度|Getangle))
  (bind _result (LocalVariables|GetResult))
  (bind _returnvalue (- _angle_2 _anglestep))
  (bind _returnvalue_2 (- _angle_3 _anglestep_2))
  (bind _returnvalue_3 (Math|Trig|Cos(Degrees) _angle_4))
  (bind _returnvalue_4 (Math|Trig|Sin(Degrees) _angle_4))
  (bind _returnvalue_5 (CallFunction|CosA _angle))
  (bind _returnvalue_6 (CallFunction|SinA _angle))
  (bind _returnvalue_7 (Math|Trig|Sin(Degrees) _returnvalue_2))
  (bind _returnvalue_8 (Math|Trig|Cos(Degrees) _returnvalue_2))
  (bind _returnvalue_9 (CallFunction|SinA _returnvalue))
  (bind _returnvalue_10 (CallFunction|CosA _returnvalue))
  (bind _returnvalue_11 (* _returnvalue_3 _inner_3))
  (bind _returnvalue_12 (* _returnvalue_4 _inner_4))
  (bind _returnvalue_13 (* _returnvalue_7 _inner_2))
  (bind _returnvalue_14 (* _returnvalue_8 _inner))
  (Utilities|FlowControl|Sequence
    (:then_0
      (LocalVariables|Setouter5 (Math|Vector|MakeVector _returnvalue_9 _returnvalue_10 (Variables|高度|Getheight)))
      (LocalVariables|Setouter6 (Math|Vector|MakeVector _returnvalue_6 _returnvalue_5 (Variables|高度|Getheight)))
      (LocalVariables|Setouter7 (Math|Vector|MakeVector _returnvalue_6 _returnvalue_5 0.0))
      (LocalVariables|Setouter8 (Math|Vector|MakeVector _returnvalue_9 _returnvalue_10 0.0)))
    (:then_1
      (LocalVariables|SetInner1 (Math|Vector|MakeVector _returnvalue_13 _returnvalue_14 (Variables|高度|Getheight)))
      (LocalVariables|SetInner2 (Math|Vector|MakeVector _returnvalue_12 _returnvalue_11 (Variables|高度|Getheight)))
      (LocalVariables|SetInner3 (Math|Vector|MakeVector _returnvalue_12 _returnvalue_11 0.0))
      (LocalVariables|SetInner4 (Math|Vector|MakeVector _returnvalue_13 _returnvalue_14 0.0)))
    (:then_2
      (Utilities|Array|AppendArray _result (select (> (Variables|半径|Getinner) 0.0) (Utilities|Array|MakeArray (Utilities|Struct|MakeCustomMeshTriangle (LocalVariables|GetInner1) (LocalVariables|Getouter5) (LocalVariables|Getouter6)) (Utilities|Struct|MakeCustomMeshTriangle (LocalVariables|Getouter6) (LocalVariables|GetInner2) (LocalVariables|GetInner1))) (Utilities|Array|MakeArray (Utilities|Struct|MakeCustomMeshTriangle (LocalVariables|GetInner1) (LocalVariables|Getouter5) (LocalVariables|Getouter6)))))
      (Utilities|Array|AppendArray _result (select (> (Variables|半径|Getinner) 0.0) (Utilities|Array|MakeArray (Utilities|Struct|MakeCustomMeshTriangle (LocalVariables|GetInner3) (LocalVariables|Getouter7) (LocalVariables|Getouter8)) (Utilities|Struct|MakeCustomMeshTriangle (LocalVariables|Getouter8) (LocalVariables|GetInner4) (LocalVariables|GetInner3))) (Utilities|Array|MakeArray (Utilities|Struct|MakeCustomMeshTriangle (LocalVariables|GetInner3) (LocalVariables|Getouter7) (LocalVariables|Getouter8)))))
      (Utilities|Array|AppendArray _result (Utilities|Array|MakeArray (Utilities|Struct|MakeCustomMeshTriangle (LocalVariables|Getouter8) (LocalVariables|Getouter7) (LocalVariables|Getouter6)) (Utilities|Struct|MakeCustomMeshTriangle (LocalVariables|Getouter6) (LocalVariables|Getouter5) (LocalVariables|Getouter8))))
      (Utilities|FlowControl|Sequence
        (:then_0
          (if (not (and bIsFirstSegment bIsLastSegment))
            (Utilities|FlowControl|Sequence
              (:then_0
                (if bIsFirstSegment
                  (Utilities|Array|AppendArray (LocalVariables|GetResult) (Utilities|Array|MakeArray (Utilities|Struct|MakeCustomMeshTriangle (LocalVariables|GetInner1) (LocalVariables|GetInner4) (LocalVariables|Getouter8)) (Utilities|Struct|MakeCustomMeshTriangle (LocalVariables|Getouter8) (LocalVariables|Getouter5) (LocalVariables|GetInner1))))))
              (:then_1
                (if bIsLastSegment
                  (Utilities|Array|AppendArray (LocalVariables|GetResult) (Utilities|Array|MakeArray (Utilities|Struct|MakeCustomMeshTriangle (LocalVariables|GetInner2) (LocalVariables|Getouter6) (LocalVariables|Getouter7)) (Utilities|Struct|MakeCustomMeshTriangle (LocalVariables|Getouter7) (LocalVariables|GetInner3) (LocalVariables|GetInner2)))))))))
        (:then_1
          (if (> (Variables|半径|Getinner) 0.0)
            (Utilities|Array|AppendArray (LocalVariables|GetResult) (Utilities|Array|MakeArray (Utilities|Struct|MakeCustomMeshTriangle (LocalVariables|GetInner4) (LocalVariables|GetInner1) (LocalVariables|GetInner2)) (Utilities|Struct|MakeCustomMeshTriangle (LocalVariables|GetInner2) (LocalVariables|GetInner3) (LocalVariables|GetInner4))))))
        (:then_2
          (return (LocalVariables|GetResult)))))))

(fn DrawSegment
  (params (from :type Float%20%28single-precision%29) (to :type Float%20%28single-precision%29) (height :type Float%20%28single-precision%29) (Value :type Linear%20Color%20Structure))
  (bind _anglestep (Variables|角度|GetangleStep))
  (bind _inner (Variables|半径|Getinner))
  (bind _data (Variables|缓存|GetData))
  (bind _anglestep_2 (Variables|角度|GetangleStep))
  (bind _hovercolor (Utilities|Struct|BreakST_3DPIEData _data))
  (bind _returnvalue (/ to _anglestep_2))
  (bind _returnvalue_2 (/ from _anglestep))
  (bind _returnvalue_3 (Math|Float|Ceil _returnvalue))
  (bind _returnvalue_4 (Math|Float|Ceil _returnvalue_2))
  (bind _returnvalue_5 (== _returnvalue_4 0))
  (bind _returnvalue_6 (== _returnvalue_3 360))
  (bind _returnvalue_7 (and _returnvalue_5 _returnvalue_6))
  (bind _returnvalue_8 (not _returnvalue_7))
  (if (and (< _inner (Variables|半径|Getouter)) (>= _inner 0.0))
    (LocalVariables|SetColor Value)
    (Variables|高度|Setheight height)
    (for _index (range _returnvalue_4 _returnvalue_3)
      (Variables|角度|Setangle (* _index (Variables|角度|GetangleStep)))
      (if (!= _index _returnvalue_4)
        (bind _triangles (CallFunction|GetSegmentTraingleList (and (== _index (+ _returnvalue_4 1)) _returnvalue_8) (and (== _index _returnvalue_3) _returnvalue_8)))
        (Utilities|Array|AppendArray (LocalVariables|GettriangleList) _triangles)))
    (bind _returnvalue_9 (AddComponent|AddProceduralMeshComponent false))
    (Utilities|Map|Add (Variables|缓存|GetcompsDegreeCenter) _returnvalue_9 (/ (+ from to) 2.0))
    (Class|ProceduralMeshComponent|CreateMeshSectionLinearColor _returnvalue_9 0 (.Vertexs (CallFunction|GetProceduralMeshData (LocalVariables|GettriangleList) (LocalVariables|GetColor))) (.Index (CallFunction|GetProceduralMeshData (LocalVariables|GettriangleList) (LocalVariables|GetColor))) (.Normals (CallFunction|GetProceduralMeshData (LocalVariables|GettriangleList) (LocalVariables|GetColor))) 0 0 0 0 (.VertexColor (CallFunction|GetProceduralMeshData (LocalVariables|GettriangleList) (LocalVariables|GetColor))) 0 true)
    (if (>= (.A (Math|Color|BreakColor (LocalVariables|GetColor))) 1.0)
      (bind _returnvalue_10 (Rendering|Material|CreateDynamicMaterialInstance "/Game/RenderTarget/M_Vertex.M_Vertex" "None" "None" :!class /Script/Engine.KismetMaterialLibrary))
      (Rendering|Material|SetScalarParameterValue _returnvalue_10 "Hover" 0.0 :!class /Script/Engine.MaterialInstanceDynamic)
      (Rendering|Material|SetMaterial _returnvalue_9 0 _returnvalue_10)
      (Rendering|Material|SetVectorParameterValue _returnvalue_10 "HoverColor" _hovercolor :!class /Script/Engine.MaterialInstanceDynamic)
      (else
        (bind _returnvalue_11 (Rendering|Material|CreateDynamicMaterialInstance "/Game/RenderTarget/M_Vertex_Translucent.M_Vertex_Translucent" "None" "None" :!class /Script/Engine.KismetMaterialLibrary))
        (Rendering|Material|SetScalarParameterValue _returnvalue_11 "Hover" 0.0 :!class /Script/Engine.MaterialInstanceDynamic)
        (Rendering|Material|SetMaterial _returnvalue_9 0 _returnvalue_11)
        (Rendering|Material|SetVectorParameterValue _returnvalue_11 "HoverColor" _hovercolor :!class /Script/Engine.MaterialInstanceDynamic)))))

(fn GetProceduralMeshData
  (params (Triangles :type Array%20of%20Custom%20Mesh%20Triangle%20Structures) (Color :type Linear%20Color%20Structure))
  (for _array_element Triangles
    (Utilities|FlowControl|Sequence
      (:then_0
        (bind _returnvalue (Utilities|Array|Add (LocalVariables|Get顶点) (.Vertex0 (Utilities|Struct|BreakCustomMeshTriangle _array_element))))
        (Utilities|Array|Add (LocalVariables|Get顶点顺序) _returnvalue))
      (:then_1
        (bind _returnvalue_2 (Utilities|Array|Add (LocalVariables|Get顶点) (.Vertex1 (Utilities|Struct|BreakCustomMeshTriangle _array_element))))
        (Utilities|Array|Add (LocalVariables|Get顶点顺序) _returnvalue_2))
      (:then_2
        (bind _returnvalue_3 (Utilities|Array|Add (LocalVariables|Get顶点) (.Vertex2 (Utilities|Struct|BreakCustomMeshTriangle _array_element))))
        (Utilities|Array|Add (LocalVariables|Get顶点顺序) _returnvalue_3)))
    (Utilities|Array|Add (LocalVariables|Get法线) (Math|Vector|Normalize (Math|Vector|CrossProduct (- (.Vertex1 (Utilities|Struct|BreakCustomMeshTriangle _array_element)) (.Vertex0 (Utilities|Struct|BreakCustomMeshTriangle _array_element))) (- (.Vertex2 (Utilities|Struct|BreakCustomMeshTriangle _array_element)) (.Vertex0 (Utilities|Struct|BreakCustomMeshTriangle _array_element))))))
    (Utilities|Array|Add (LocalVariables|Get顶点颜色) Color))
  (return (LocalVariables|Get顶点) (LocalVariables|Get顶点顺序) (LocalVariables|Get法线) (LocalVariables|Get顶点颜色)))

(fn HoverComp
  (params (Key :type Procedural%20Mesh%20Component%20Object%20Reference%20%28by%20ref%29))
  (bind _hoverinterval (Variables|半径|GethoverInterval))
  (bind _compsdegreecenter (Variables|缓存|GetcompsDegreeCenter))
  (bind _value (Utilities|Map|Find _compsdegreecenter Key))
  (Transformation|SetRelativeLocation Key (Math|Vector|MakeVector (* _hoverinterval (Math|Trig|Sin(Degrees) _value)) (* (Math|Trig|Cos(Degrees) _value) _hoverinterval) 0.0) false false))

(fn NotifyElementTipsLoc
  (bind _compsdegreecenter (Variables|缓存|GetcompsDegreeCenter))
  (bind _outer (Variables|半径|Getouter))
  (bind _keys (Utilities|Map|Keys _compsdegreecenter))
  (for (_array_element _array_index) _keys
    (Utilities|IsValid _array_element
      (:Is%20Valid
        (Utilities|Array|Add (LocalVariables|GetCenterPos) (+ (Math|Vector|MakeVector (* (Math|Trig|Sin(Degrees) (.Value (Utilities|Map|Find _compsdegreecenter _array_element))) (Math|Float|SelectFloat (+ _outer (Variables|半径|GethoverInterval)) _outer (== (Variables|Default|GetLastComp) _array_element))) (* (Math|Float|SelectFloat (+ _outer (Variables|半径|GethoverInterval)) _outer (== (Variables|Default|GetLastComp) _array_element)) (Math|Trig|Cos(Degrees) (.Value (Utilities|Map|Find _compsdegreecenter _array_element)))) (.Height (Utilities|Struct|BreakST_3DPIESegementData (Utilities|Array|Get(acopy) (.segementData (Utilities|Struct|BreakST_3DPIEData (Variables|缓存|GetData))) _array_index)))) (Transformation|GetActorLocation))))))
  (Default|CallOnCenterPosGet (LocalVariables|GetCenterPos) (CallFunction|GetCameraMinimalViewInfo (Variables|缓存|GetaspectRatio)) (Variables|Default|GetSceneCaptureComponent2D)))

(fn GetCameraMinimalViewInfo
  (params (Aspect%20Ratio :type Float%20%28single-precision%29))
  (bind _scenecapturecomponent2d (Variables|Default|GetSceneCaptureComponent2D))
  (return (Utilities|Struct|MakeMinimalViewInfo (Transformation|GetWorldLocation _scenecapturecomponent2d) (Transformation|GetWorldRotation _scenecapturecomponent2d) (Variables|/Script/Engine.SceneCaptureComponent2D|GetFOVAngle (Variables|Default|GetSceneCaptureComponent2D)) 512.0 0.0 2097152.0 Aspect%20Ratio true true "Perspective" 0.0 "(bOverride_TemperatureType=False,bOverride_WhiteTemp=False,bOverride_WhiteTint=False,bOverride_ColorSaturation=False,bOverride_ColorContrast=False,bOverride_ColorGamma=False,bOverride_ColorGain=False,bOverride_ColorOffset=False,bOverride_ColorSaturationShadows=False,bOverride_ColorContrastShadows=False,bOverride_ColorGammaShadows=False,bOverride_ColorGainShadows=False,bOverride_ColorOffsetShadows=False,bOverride_ColorSaturationMidtones=False,bOverride_ColorContrastMidtones=False,bOverride_ColorGammaMidtones=False,bOverride_ColorGainMidtones=False,bOverride_ColorOffsetMidtones=False,bOverride_ColorSaturationHighlights=False,bOverride_ColorContrastHighlights=False,bOverride_ColorGammaHighlights=False,bOverride_ColorGainHighlights=False,bOverride_ColorOffsetHighlights=False,bOverride_ColorCorrectionShadowsMax=False,bOverride_ColorCorrectionHighlightsMin=False,bOverride_BlueCorrection=False,bOverride_ExpandGamut=False,bOverride_ToneCurveAmount=False,bOverride_FilmWhitePoint=False,bOverride_FilmSaturation=False,bOverride_FilmChannelMixerRed=False,bOverride_FilmChannelMixerGreen=False,bOverride_FilmChannelMixerBlue=False,bOverride_FilmContrast=False,bOverride_FilmDynamicRange=False,bOverride_FilmHealAmount=False,bOverride_FilmToeAmount=False,bOverride_FilmShadowTint=False,bOverride_FilmShadowTintBlend=False,bOverride_FilmShadowTintAmount=False,bOverride_FilmSlope=False,bOverride_FilmToe=False,bOverride_FilmShoulder=False,bOverride_FilmBlackClip=False,bOverride_FilmWhiteClip=False,bOverride_SceneColorTint=False,bOverride_SceneFringeIntensity=False,bOverride_ChromaticAberrationStartOffset=False,bOverride_AmbientCubemapTint=False,bOverride_AmbientCubemapIntensity=False,bOverride_BloomMethod=False,bOverride_BloomIntensity=False,bOverride_BloomThreshold=False,bOverride_Bloom1Tint=False,bOverride_Bloom1Size=False,bOverride_Bloom2Size=False,bOverride_Bloom2Tint=False,bOverride_Bloom3Tint=False,bOverride_Bloom3Size=False,bOverride_Bloom4Tint=False,bOverride_Bloom4Size=False,bOverride_Bloom5Tint=False,bOverride_Bloom5Size=False,bOverride_Bloom6Tint=False,bOverride_Bloom6Size=False,bOverride_BloomSizeScale=False,bOverride_BloomConvolutionTexture=False,bOverride_BloomConvolutionSize=False,bOverride_BloomConvolutionCenterUV=False,bOverride_BloomConvolutionPreFilterMin=False,bOverride_BloomConvolutionPreFilterMax=False,bOverride_BloomConvolutionPreFilterMult=False,bOverride_BloomConvolutionBufferScale=False,bOverride_BloomDirtMaskIntensity=False,bOverride_BloomDirtMaskTint=False,bOverride_BloomDirtMask=False,bOverride_CameraShutterSpeed=False,bOverride_CameraISO=False,bOverride_AutoExposureMethod=False,bOverride_AutoExposureLowPercent=False,bOverride_AutoExposureHighPercent=False,bOverride_AutoExposureMinBrightness=False,bOverride_AutoExposureMaxBrightness=False,bOverride_AutoExposureSpeedUp=False,bOverride_AutoExposureSpeedDown=False,bOverride_AutoExposureBias=False,bOverride_AutoExposureBiasCurve=False,bOverride_AutoExposureMeterMask=False,bOverride_AutoExposureApplyPhysicalCameraExposure=False,bOverride_HistogramLogMin=False,bOverride_HistogramLogMax=False,bOverride_LensFlareIntensity=False,bOverride_LensFlareTint=False,bOverride_LensFlareTints=False,bOverride_LensFlareBokehSize=False,bOverride_LensFlareBokehShape=False,bOverride_LensFlareThreshold=False,bOverride_VignetteIntensity=False,bOverride_GrainIntensity=False,bOverride_GrainJitter=False,bOverride_AmbientOcclusionIntensity=False,bOverride_AmbientOcclusionStaticFraction=False,bOverride_AmbientOcclusionRadius=False,bOverride_AmbientOcclusionFadeDistance=False,bOverride_AmbientOcclusionFadeRadius=False,bOverride_AmbientOcclusionRadiusInWS=False,bOverride_AmbientOcclusionPower=False,bOverride_AmbientOcclusionBias=False,bOverride_AmbientOcclusionQuality=False,bOverride_AmbientOcclusionMipBlend=False,bOverride_AmbientOcclusionMipScale=False,bOverride_AmbientOcclusionMipThreshold=False,bOverride_AmbientOcclusionTemporalBlendWeight=False,bOverride_RayTracingAO=False,bOverride_RayTracingAOSamplesPerPixel=False,bOverride_RayTracingAOIntensity=False,bOverride_RayTracingAORadius=False,bOverride_LPVIntensity=False,bOverride_LPVDirectionalOcclusionIntensity=False,bOverride_LPVDirectionalOcclusionRadius=False,bOverride_LPVDiffuseOcclusionExponent=False,bOverride_LPVSpecularOcclusionExponent=False,bOverride_LPVDiffuseOcclusionIntensity=False,bOverride_LPVSpecularOcclusionIntensity=False,bOverride_LPVSize=False,bOverride_LPVSecondaryOcclusionIntensity=False,bOverride_LPVSecondaryBounceIntensity=False,bOverride_LPVGeometryVolumeBias=False,bOverride_LPVVplInjectionBias=False,bOverride_LPVEmissiveInjectionIntensity=False,bOverride_LPVFadeRange=False,bOverride_LPVDirectionalOcclusionFadeRange=False,bOverride_IndirectLightingColor=False,bOverride_IndirectLightingIntensity=False,bOverride_ColorGradingIntensity=False,bOverride_ColorGradingLUT=False,bOverride_DepthOfFieldFocalDistance=False,bOverride_DepthOfFieldFstop=False,bOverride_DepthOfFieldMinFstop=False,bOverride_DepthOfFieldBladeCount=False,bOverride_DepthOfFieldSensorWidth=False,bOverride_DepthOfFieldDepthBlurRadius=False,bOverride_DepthOfFieldDepthBlurAmount=False,bOverride_DepthOfFieldFocalRegion=False,bOverride_DepthOfFieldNearTransitionRegion=False,bOverride_DepthOfFieldFarTransitionRegion=False,bOverride_DepthOfFieldScale=False,bOverride_DepthOfFieldNearBlurSize=False,bOverride_DepthOfFieldFarBlurSize=False,bOverride_MobileHQGaussian=False,bOverride_DepthOfFieldOcclusion=False,bOverride_DepthOfFieldSkyFocusDistance=False,bOverride_DepthOfFieldVignetteSize=False,bOverride_MotionBlurAmount=False,bOverride_MotionBlurMax=False,bOverride_MotionBlurTargetFPS=False,bOverride_MotionBlurPerObjectSize=False,bOverride_ScreenPercentage=False,bOverride_ScreenSpaceReflectionIntensity=False,bOverride_ScreenSpaceReflectionQuality=False,bOverride_ScreenSpaceReflectionMaxRoughness=False,bOverride_ScreenSpaceReflectionRoughnessScale=False,bOverride_ReflectionsType=False,bOverride_RayTracingReflectionsMaxRoughness=False,bOverride_RayTracingReflectionsMaxBounces=False,bOverride_RayTracingReflectionsSamplesPerPixel=False,bOverride_RayTracingReflectionsShadows=False,bOverride_RayTracingReflectionsTranslucency=False,bOverride_TranslucencyType=False,bOverride_RayTracingTranslucencyMaxRoughness=False,bOverride_RayTracingTranslucencyRefractionRays=False,bOverride_RayTracingTranslucencySamplesPerPixel=False,bOverride_RayTracingTranslucencyShadows=False,bOverride_RayTracingTranslucencyRefraction=False,bOverride_RayTracingGI=False,bOverride_RayTracingGIMaxBounces=False,bOverride_RayTracingGISamplesPerPixel=False,bOverride_PathTracingMaxBounces=False,bOverride_PathTracingSamplesPerPixel=False,bOverride_PathTracingFilterWidth=False,bOverride_PathTracingEnableEmissive=False,bOverride_PathTracingMaxPathExposure=False,bOverride_PathTracingEnableDenoiser=False,bMobileHQGaussian=False,BloomMethod=BM_SOG,AutoExposureMethod=AEM_Histogram,TemperatureType=TEMP_WhiteBalance,WhiteTemp=6500.000000,WhiteTint=0.000000,ColorSaturation=(X=1.000000,Y=1.000000,Z=1.000000,W=1.000000),ColorContrast=(X=1.000000,Y=1.000000,Z=1.000000,W=1.000000),ColorGamma=(X=1.000000,Y=1.000000,Z=1.000000,W=1.000000),ColorGain=(X=1.000000,Y=1.000000,Z=1.000000,W=1.000000),ColorOffset=(X=0.000000,Y=0.000000,Z=0.000000,W=0.000000),ColorSaturationShadows=(X=1.000000,Y=1.000000,Z=1.000000,W=1.000000),ColorContrastShadows=(X=1.000000,Y=1.000000,Z=1.000000,W=1.000000),ColorGammaShadows=(X=1.000000,Y=1.000000,Z=1.000000,W=1.000000),ColorGainShadows=(X=1.000000,Y=1.000000,Z=1.000000,W=1.000000),ColorOffsetShadows=(X=0.000000,Y=0.000000,Z=0.000000,W=0.000000),ColorSaturationMidtones=(X=1.000000,Y=1.000000,Z=1.000000,W=1.000000),ColorContrastMidtones=(X=1.000000,Y=1.000000,Z=1.000000,W=1.000000),ColorGammaMidtones=(X=1.000000,Y=1.000000,Z=1.000000,W=1.000000),ColorGainMidtones=(X=1.000000,Y=1.000000,Z=1.000000,W=1.000000),ColorOffsetMidtones=(X=0.000000,Y=0.000000,Z=0.000000,W=0.000000),ColorSaturationHighlights=(X=1.000000,Y=1.000000,Z=1.000000,W=1.000000),ColorContrastHighlights=(X=1.000000,Y=1.000000,Z=1.000000,W=1.000000),ColorGammaHighlights=(X=1.000000,Y=1.000000,Z=1.000000,W=1.000000),ColorGainHighlights=(X=1.000000,Y=1.000000,Z=1.000000,W=1.000000),ColorOffsetHighlights=(X=0.000000,Y=0.000000,Z=0.000000,W=0.000000),ColorCorrectionHighlightsMin=0.500000,ColorCorrectionShadowsMax=0.090000,BlueCorrection=0.600000,ExpandGamut=1.000000,ToneCurveAmount=1.000000,FilmSlope=0.880000,FilmToe=0.550000,FilmShoulder=0.260000,FilmBlackClip=0.000000,FilmWhiteClip=0.040000,FilmWhitePoint=(R=1.000000,G=1.000000,B=1.000000,A=1.000000),FilmShadowTint=(R=1.000000,G=1.000000,B=1.000000,A=1.000000),FilmShadowTintBlend=0.500000,FilmShadowTintAmount=0.000000,FilmSaturation=1.000000,FilmChannelMixerRed=(R=1.000000,G=0.000000,B=0.000000,A=1.000000),FilmChannelMixerGreen=(R=0.000000,G=1.000000,B=0.000000,A=1.000000),FilmChannelMixerBlue=(R=0.000000,G=0.000000,B=1.000000,A=1.000000),FilmContrast=0.030000,FilmToeAmount=1.000000,FilmHealAmount=1.000000,FilmDynamicRange=4.000000,SceneColorTint=(R=1.000000,G=1.000000,B=1.000000,A=1.000000),SceneFringeIntensity=0.000000,ChromaticAberrationStartOffset=0.000000,BloomIntensity=0.675000,BloomThreshold=-1.000000,BloomSizeScale=4.000000,Bloom1Size=0.300000,Bloom2Size=1.000000,Bloom3Size=2.000000,Bloom4Size=10.000000,Bloom5Size=30.000000,Bloom6Size=64.000000,Bloom1Tint=(R=0.346500,G=0.346500,B=0.346500,A=1.000000),Bloom2Tint=(R=0.138000,G=0.138000,B=0.138000,A=1.000000),Bloom3Tint=(R=0.117600,G=0.117600,B=0.117600,A=1.000000),Bloom4Tint=(R=0.066000,G=0.066000,B=0.066000,A=1.000000),Bloom5Tint=(R=0.066000,G=0.066000,B=0.066000,A=1.000000),Bloom6Tint=(R=0.061000,G=0.061000,B=0.061000,A=1.000000),BloomConvolutionSize=1.000000,BloomConvolutionTexture=None,BloomConvolutionCenterUV=(X=0.500000,Y=0.500000),BloomConvolutionPreFilterMin=7.000000,BloomConvolutionPreFilterMax=15000.000000,BloomConvolutionPreFilterMult=15.000000,BloomConvolutionBufferScale=0.133000,BloomDirtMask=None,BloomDirtMaskIntensity=0.000000,BloomDirtMaskTint=(R=0.500000,G=0.500000,B=0.500000,A=1.000000),AmbientCubemapTint=(R=1.000000,G=1.000000,B=1.000000,A=1.000000),AmbientCubemapIntensity=1.000000,AmbientCubemap=None,CameraShutterSpeed=60.000000,CameraISO=100.000000,DepthOfFieldFstop=4.000000,DepthOfFieldMinFstop=1.200000,DepthOfFieldBladeCount=5,AutoExposureBias=1.000000,AutoExposureBiasBackup=0.000000,bOverride_AutoExposureBiasBackup=False,AutoExposureApplyPhysicalCameraExposure=True,AutoExposureBiasCurve=None,AutoExposureMeterMask=None,AutoExposureLowPercent=10.000000,AutoExposureHighPercent=90.000000,AutoExposureMinBrightness=0.030000,AutoExposureMaxBrightness=8.000000,AutoExposureSpeedUp=3.000000,AutoExposureSpeedDown=1.000000,HistogramLogMin=-8.000000,HistogramLogMax=4.000000,LensFlareIntensity=1.000000,LensFlareTint=(R=1.000000,G=1.000000,B=1.000000,A=1.000000),LensFlareBokehSize=3.000000,LensFlareThreshold=8.000000,LensFlareBokehShape=None,LensFlareTints[0]=(R=1.000000,G=0.800000,B=0.400000,A=0.600000),LensFlareTints[1]=(R=1.000000,G=1.000000,B=0.600000,A=0.530000),LensFlareTints[2]=(R=0.800000,G=0.800000,B=1.000000,A=0.460000),LensFlareTints[3]=(R=0.500000,G=1.000000,B=0.400000,A=0.390000),LensFlareTints[4]=(R=0.500000,G=0.800000,B=1.000000,A=0.310000),LensFlareTints[5]=(R=0.900000,G=1.000000,B=0.800000,A=0.270000),LensFlareTints[6]=(R=1.000000,G=0.800000,B=0.400000,A=0.220000),LensFlareTints[7]=(R=0.900000,G=0.700000,B=0.700000,A=0.150000),VignetteIntensity=0.400000,GrainJitter=0.000000,GrainIntensity=0.000000,AmbientOcclusionIntensity=0.500000,AmbientOcclusionStaticFraction=1.000000,AmbientOcclusionRadius=200.000000,AmbientOcclusionRadiusInWS=False,AmbientOcclusionFadeDistance=8000.000000,AmbientOcclusionFadeRadius=5000.000000,AmbientOcclusionPower=2.000000,AmbientOcclusionBias=3.000000,AmbientOcclusionQuality=50.000000,AmbientOcclusionMipBlend=0.600000,AmbientOcclusionMipScale=1.700000,AmbientOcclusionMipThreshold=0.010000,AmbientOcclusionTemporalBlendWeight=0.100000,RayTracingAO=True,RayTracingAOSamplesPerPixel=1,RayTracingAOIntensity=1.000000,RayTracingAORadius=200.000000,IndirectLightingColor=(R=1.000000,G=1.000000,B=1.000000,A=1.000000),IndirectLightingIntensity=1.000000,RayTracingGIType=Disabled,RayTracingGIMaxBounces=1,RayTracingGISamplesPerPixel=4,ColorGradingIntensity=1.000000,ColorGradingLUT=None,DepthOfFieldSensorWidth=24.576000,DepthOfFieldFocalDistance=0.000000,DepthOfFieldDepthBlurAmount=1.000000,DepthOfFieldDepthBlurRadius=0.000000,DepthOfFieldFocalRegion=0.000000,DepthOfFieldNearTransitionRegion=300.000000,DepthOfFieldFarTransitionRegion=500.000000,DepthOfFieldScale=0.000000,DepthOfFieldNearBlurSize=15.000000,DepthOfFieldFarBlurSize=15.000000,DepthOfFieldOcclusion=0.400000,DepthOfFieldSkyFocusDistance=0.000000,DepthOfFieldVignetteSize=200.000000,MotionBlurAmount=0.500000,MotionBlurMax=5.000000,MotionBlurTargetFPS=30,MotionBlurPerObjectSize=0.500000,LPVIntensity=1.000000,LPVVplInjectionBias=0.640000,LPVSize=5312.000000,LPVSecondaryOcclusionIntensity=0.000000,LPVSecondaryBounceIntensity=0.000000,LPVGeometryVolumeBias=0.384000,LPVEmissiveInjectionIntensity=1.000000,LPVDirectionalOcclusionIntensity=0.000000,LPVDirectionalOcclusionRadius=8.000000,LPVDiffuseOcclusionExponent=1.000000,LPVSpecularOcclusionExponent=7.000000,LPVDiffuseOcclusionIntensity=1.000000,LPVSpecularOcclusionIntensity=1.000000,ReflectionsType=RayTracing,ScreenSpaceReflectionIntensity=100.000000,ScreenSpaceReflectionQuality=50.000000,ScreenSpaceReflectionMaxRoughness=0.600000,RayTracingReflectionsMaxRoughness=0.600000,RayTracingReflectionsMaxBounces=1,RayTracingReflectionsSamplesPerPixel=1,RayTracingReflectionsShadows=Hard_shadows,RayTracingReflectionsTranslucency=False,TranslucencyType=Raster,RayTracingTranslucencyMaxRoughness=0.600000,RayTracingTranslucencyRefractionRays=3,RayTracingTranslucencySamplesPerPixel=1,RayTracingTranslucencyShadows=Hard_shadows,RayTracingTranslucencyRefraction=True,PathTracingMaxBounces=32,PathTracingSamplesPerPixel=16384,PathTracingFilterWidth=3.000000,PathTracingEnableEmissive=True,PathTracingMaxPathExposure=30.000000,PathTracingEnableDenoiser=True,LPVFadeRange=0.000000,LPVDirectionalOcclusionFadeRange=0.000000,ScreenPercentage=100.000000,WeightedBlendables=(Array=))" "(X=0.000000,Y=0.000000)")))

(fn InitSegement
  (params (Data :type ST%203DPIE%20Data%20Structure%20%28by%20ref%29))
  (bind (_inner _outter _hoverinterval _hovercolor _segementdata) (Utilities|Struct|BreakST_3DPIEData Data))
  (Variables|半径|Setinner _inner)
  (Variables|半径|Setouter _outter)
  (Variables|半径|SethoverInterval _hoverinterval)
  (for _array_element _segementdata
    (CallFunction|DrawSegment (* (LocalVariables|GetTotalPercent) 3.6e+02) (* (+ (.Percentage (Utilities|Struct|BreakST_3DPIESegementData _array_element)) (LocalVariables|GetTotalPercent)) 3.6e+02) (.Height (Utilities|Struct|BreakST_3DPIESegementData _array_element)) (.Color (Utilities|Struct|BreakST_3DPIESegementData _array_element)))
    (LocalVariables|SetTotalPercent (+ (.Percentage (Utilities|Struct|BreakST_3DPIESegementData _array_element)) (LocalVariables|GetTotalPercent)))))